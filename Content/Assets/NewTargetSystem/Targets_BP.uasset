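; Destructible target that plane missiles and projectiles damage for points.
; On hit, it casts for Missile_NT or Projectile_BP and applies the matching damage from player pawn 0's DamageSystem to its HealthSystem.
; At zero health it destroys itself and adds a point to the hitting object's MainPlane_BP owner.
; A separate DestroyTargetBp function, not called here, removes the first BP_target_marker found.
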(event `self.ReceiveHit`
  (params (MyComp :type "PrimitiveComponent Object Reference") (Other :type "Actor Object Reference") (OtherComp :type "PrimitiveComponent Object Reference") (bSelfMoved :type Boolean) (HitLocation :type "Vector Structure") (HitNormal :type "Vector Structure") (NormalImpulse :type "Vector Structure") (Hit :type "HitResult Structure (by ref)"))
  (bind _returnvalue (`self.GetOwner` Other))
  (bind _healthsystem (`self.HealthSystem`))
  (bind _healthsystem_2 (`self.HealthSystem`))
  ;[1 1 1] Checks hit from bullets
  ;[1 1 1] Checks hit from missiles
  (`|ExecutionSequence`
    (:`then_0`
      (cast `/Game/Assets/NewTargetSystem/Missile_NT` Other)
      (`HealthSystem.TakeDamage` _healthsystem (`DamageSystem.GetMissileDamage` (`self.GetComponentByClass` (`GameplayStatics.GetPlayerPawn` 0) "/Script/SkyFrontier.DamageSystem")))
      (if (<= (`HealthSystem.GetHealth` _healthsystem) 0.0)
        (`self.K2_DestroyActor`)
        ;[1 1 1] Add points to player
        (bind _asmain_plane_bp (cast `/Game/Assets/NormieAsset/MainPlane_BP` _returnvalue :!label _label))
        (`PointsComponent.AddPoints` (`/Game/Assets/NormieAsset/MainPlane_BP.Points` _asmain_plane_bp) 1)
        (`KismetSystemLibrary.PrintString` (`KismetStringLibrary.Concat_StrStr` (`KismetSystemLibrary.GetDisplayName` _returnvalue) " Got Points") true true (struct :`G` 0.042901 :`B` 1.0 :`A` 1.0))))
    (:`then_1`
      (cast `/Game/Assets/Projectiles/Projectile_BP` Other)
      (`HealthSystem.TakeDamage` _healthsystem_2 (`DamageSystem.GetShootingDamage` (`self.GetComponentByClass` (`GameplayStatics.GetPlayerPawn` 0) "/Script/SkyFrontier.DamageSystem")))
      (if (<= (`HealthSystem.GetHealth` _healthsystem_2) 0.0)
        (`self.K2_DestroyActor`)
        (goto _label)))))

(fn `DestroyTargetBp`
  (bind _returnvalue (`GameplayStatics.GetActorOfClass` "/Game/Assets/NewTargetSystem/BP_target_marker.BP_target_marker_C"))
  (`/Engine/EditorBlueprintResources/StandardMacros.IsValid` _returnvalue
    (:`Is Valid`
      (`self.K2_DestroyActor` _returnvalue))))

(fn `UserConstructionScript`)