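; BP_East_Missile_P270 is a missile Blueprint that exposes control events for its thruster effect and animated fins, with no flight or damage logic in its graphs.
; BeginPlay caches the mesh's ABP_East_Missile_P270 instance, and the events write fin values into it.
; Eight deflection events map normalized input to symmetric angles for front and rear fins.
; One fold event drives all fins, negating the angle for fins 1 and 3.
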(event `self.ReceiveBeginPlay`
  (bind _asabp_east_missile_p270 (cast `/Game/Assets/Projectiles/Missile/VigilanteContent/Projectiles/East_Missile_P270/ABP_East_Missile_P270` (`SkeletalMeshComponent.GetAnimInstance` (`self.SkeletalMesh`))))
  (set `self.AnimInstance` _asabp_east_missile_p270))

(event `SetEngineState`
  (params (bEngineActive :type Boolean))
  ;[1 1 1] Set engine state
  (`ActorComponent.SetActive` (`self.ThrusterFX`) bEngineActive true))

(event `SetFinFront1Angle`
  (params (Angle :type "Float (double-precision)"))
  (set `/Game/Assets/Projectiles/Missile/VigilanteContent/Projectiles/East_Missile_P270/ABP_East_Missile_P270.FinF1Angle` (`KismetMathLibrary.MapRangeClamped` Angle -1.0 1.0 -45.0 45.0) (`self.AnimInstance`)))

(event `SetFinRear1Angle`
  (params (Angle :type "Float (double-precision)"))
  (set `/Game/Assets/Projectiles/Missile/VigilanteContent/Projectiles/East_Missile_P270/ABP_East_Missile_P270.FinR1Angle` (`KismetMathLibrary.MapRangeClamped` Angle -1.0 1.0 -45.0 45.0) (`self.AnimInstance`)))

(event `SetFinFront2Angle`
  (params (Angle :type "Float (double-precision)"))
  (set `/Game/Assets/Projectiles/Missile/VigilanteContent/Projectiles/East_Missile_P270/ABP_East_Missile_P270.FinF2Angle` (`KismetMathLibrary.MapRangeClamped` Angle -1.0 1.0 -45.0 45.0) (`self.AnimInstance`)))

(event `SetFinRear2Angle`
  (params (Angle :type "Float (double-precision)"))
  (set `/Game/Assets/Projectiles/Missile/VigilanteContent/Projectiles/East_Missile_P270/ABP_East_Missile_P270.FinR2Angle` (`KismetMathLibrary.MapRangeClamped` Angle -1.0 1.0 -45.0 45.0) (`self.AnimInstance`)))

(event `SetFinFront3Angle`
  (params (Angle :type "Float (double-precision)"))
  (set `/Game/Assets/Projectiles/Missile/VigilanteContent/Projectiles/East_Missile_P270/ABP_East_Missile_P270.FinF3Angle` (`KismetMathLibrary.MapRangeClamped` Angle -1.0 1.0 -45.0 45.0) (`self.AnimInstance`)))

(event `SetFinRear3Angle`
  (params (Angle :type "Float (double-precision)"))
  (set `/Game/Assets/Projectiles/Missile/VigilanteContent/Projectiles/East_Missile_P270/ABP_East_Missile_P270.FinR3Angle` (`KismetMathLibrary.MapRangeClamped` Angle -1.0 1.0 -45.0 45.0) (`self.AnimInstance`)))

(event `SetFinFront4Angle`
  (params (Angle :type "Float (double-precision)"))
  (set `/Game/Assets/Projectiles/Missile/VigilanteContent/Projectiles/East_Missile_P270/ABP_East_Missile_P270.FinF4Angle` (`KismetMathLibrary.MapRangeClamped` Angle -1.0 1.0 -45.0 45.0) (`self.AnimInstance`)))

(event `SetFinRear4Angle`
  (params (Angle :type "Float (double-precision)"))
  (set `/Game/Assets/Projectiles/Missile/VigilanteContent/Projectiles/East_Missile_P270/ABP_East_Missile_P270.FinR4Angle` (`KismetMathLibrary.MapRangeClamped` Angle -1.0 1.0 -45.0 45.0) (`self.AnimInstance`)))

(event `SetFinsFold`
  (params (Angle :type "Float (double-precision)"))
  (bind _returnvalue (`KismetMathLibrary.MapRangeClamped` Angle 0.0 1.0 0.0 90.0))
  (bind _animinstance (`self.AnimInstance`))
  (bind _animinstance_2 (`self.AnimInstance`))
  (`|ExecutionSequence`
    (:`then_0`
      (bind _output_get (set `/Game/Assets/Projectiles/Missile/VigilanteContent/Projectiles/East_Missile_P270/ABP_East_Missile_P270.FinF2Fold` _returnvalue _animinstance))
      (bind _output_get_2 (set `/Game/Assets/Projectiles/Missile/VigilanteContent/Projectiles/East_Missile_P270/ABP_East_Missile_P270.FinF4Fold` _output_get _animinstance))
      (bind _output_get_3 (set `/Game/Assets/Projectiles/Missile/VigilanteContent/Projectiles/East_Missile_P270/ABP_East_Missile_P270.FinR2Fold` _output_get_2 _animinstance))
      (set `/Game/Assets/Projectiles/Missile/VigilanteContent/Projectiles/East_Missile_P270/ABP_East_Missile_P270.FinR4Fold` _output_get_3 _animinstance))
    (:`then_1`
      (bind _output_get_4 (set `/Game/Assets/Projectiles/Missile/VigilanteContent/Projectiles/East_Missile_P270/ABP_East_Missile_P270.FinF1Fold` (* _returnvalue -1.0) _animinstance_2))
      (bind _output_get_5 (set `/Game/Assets/Projectiles/Missile/VigilanteContent/Projectiles/East_Missile_P270/ABP_East_Missile_P270.FinF3Fold` _output_get_4 _animinstance_2))
      (bind _output_get_6 (set `/Game/Assets/Projectiles/Missile/VigilanteContent/Projectiles/East_Missile_P270/ABP_East_Missile_P270.FinR1Fold` _output_get_5 _animinstance_2))
      (set `/Game/Assets/Projectiles/Missile/VigilanteContent/Projectiles/East_Missile_P270/ABP_East_Missile_P270.FinR3Fold` _output_get_6 _animinstance_2))))

(fn `UserConstructionScript`)