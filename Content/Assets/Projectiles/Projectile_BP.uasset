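; Projectile Blueprint that launches from its owner and destroys itself on hitting any other actor.
; The construction script sets the ProjectileMovement initial speed to its max speed.
; On BeginPlay, the physics Box adds the owner's velocity to its own and ignores the owner when moving.
; Tick reapplies a fixed lifespan every frame, so the expiry timer keeps restarting while the actor ticks.
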(event `self.ReceiveBeginPlay`
  (`PrimitiveComponent.SetPhysicsLinearVelocity` (`self.Box`) (`self.GetVelocity` (`self.GetOwner`)) true "None")
  (`PrimitiveComponent.IgnoreActorWhenMoving` (`self.Box`) (`self.GetOwner`) true))

(event `self.ReceiveTick`
  (params (DeltaSeconds :type "Float (single-precision)"))
  (`self.SetLifeSpan` 6.0))

(event `self.ReceiveHit`
  (params (MyComp :type "PrimitiveComponent Object Reference") (Other :type "Actor Object Reference") (OtherComp :type "PrimitiveComponent Object Reference") (bSelfMoved :type Boolean) (HitLocation :type "Vector Structure") (HitNormal :type "Vector Structure") (NormalImpulse :type "Vector Structure") (Hit :type "HitResult Structure (by ref)"))
  (if (not (== (`.HitActor` (`GameplayStatics.BreakHitResult` Hit)) (`self.GetOwner`)))
    (`self.K2_DestroyActor`)))

(fn `UserConstructionScript`
  (bind _projectilemovement (`self.ProjectileMovement`))
  (set `ProjectileMovementComponent.InitialSpeed` (`MovementComponent.GetMaxSpeed` _projectilemovement) _projectilemovement))