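; Game mode Blueprint that tracks a two-player score race toward a Goal value.
; On Tick, it casts each player's pawn to Test_anim and, after a two-second Delay, copies the points from its Points component into that player's score and prints it in green or red.
; It also compares both scores to Goal every tick and prints a win message for any player who has reached it.
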(event `self.ReceiveTick`
  (params (DeltaSeconds :type "Float (single-precision)"))
  (bind _goal (`self.Goal`))
  (`|ExecutionSequence`
    (:`then_0`
      (bind _astest_anim (cast `/Game/Assets/NormieAsset/Test_anim` (`GameplayStatics.GetPlayerPawn` 0)))
      (`KismetSystemLibrary.Delay` 2.0)
      (bind _returnvalue (`PointsComponent.GetPoints` (`/Game/Assets/NormieAsset/Test_anim.Points` _astest_anim)))
      (set `self.Player1Score` _returnvalue)
      (`KismetSystemLibrary.PrintString` (`KismetStringLibrary.Conv_IntToString` _returnvalue) true true (struct :`R` 0.122594 :`G` 1.0 :`A` 1.0)))
    (:`then_1`
      (bind _astest_anim_2 (cast `/Game/Assets/NormieAsset/Test_anim` (`GameplayStatics.GetPlayerPawn` 1)))
      (`KismetSystemLibrary.Delay` 2.0)
      (bind _returnvalue_2 (`PointsComponent.GetPoints` (`/Game/Assets/NormieAsset/Test_anim.Points` _astest_anim_2)))
      (set `self.Player2Score` _returnvalue_2)
      (`KismetSystemLibrary.PrintString` (`KismetStringLibrary.Conv_IntToString` _returnvalue_2) true true (struct :`R` 1.0 :`B` 0.102424 :`A` 1.0)))
    (:`then_2`
      (if (>= (`self.Player2Score`) _goal)
        (`KismetSystemLibrary.PrintString` "Player 2 Won!")))
    (:`then_3`
      (if (>= (`self.Player1Score`) _goal)
        (`KismetSystemLibrary.PrintString` "Player 1 Won!")))))

(fn `UserConstructionScript`)