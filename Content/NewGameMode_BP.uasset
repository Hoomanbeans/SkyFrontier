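; NewGameMode_BP is a game mode that respawns the player's Test_anim pawn after it is destroyed.
; On BeginPlay it casts player pawn 0 to Test_anim and binds to its OnDestroyed event.
; On destruction it waits briefly, spawns a new Test_anim at SpawnTransform and has the player controller possess it.
; It then calls Respawn to bind the new pawn, so the cycle repeats.
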(event `Respawn`
  (bind _astest_anim (cast `/Game/Assets/NormieAsset/Test_anim` (`GameplayStatics.GetPlayerPawn` 0) :!label _label))
  (add `self.OnDestroyed` _astest_anim (delegate `OnDestroyed_Event_0`)))

(event `self.ReceiveBeginPlay`
  (goto _label))

(event `OnDestroyed_Event_0` :!signature `self.OnDestroyed`
  (params (DestroyedActor :type "Actor Object Reference"))
  (`KismetSystemLibrary.Delay` 2.0)
  (bind _returnvalue (`|SpawnActorFromClass` "/Game/Assets/NormieAsset/Test_anim.Test_anim_C" (`self.Spawn Transform`) "Undefined" "OverrideRootScale" null null))
  (`Controller.Possess` (`GameplayStatics.GetPlayerController` 0) _returnvalue)
  (`self.Respawn`))

(fn `UserConstructionScript`)