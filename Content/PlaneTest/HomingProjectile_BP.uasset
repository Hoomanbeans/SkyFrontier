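; A homing projectile that seeks Targets_BP actors, destroying itself and whatever actor it hits.
; It ignores its instigator while moving and re-runs target finding every half second to update ProjectileMovement's homing component.
; TargetFinding scans all targets against a stored ClosestDistance that it never resets, printing each new closest.
; Tick re-applies a one-second lifespan every frame, continually restarting that timer.
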(event `Travel To Target`
  (bind _projectilemovement (`self.ProjectileMovement`))
  (bind _homingtarget (`self.TargetFinding`))
  (set `ProjectileMovementComponent.HomingTargetComponent` _homingtarget _projectilemovement)
  (set `ProjectileMovementComponent.bIsHomingProjectile` true _projectilemovement))

(event `self.ReceiveBeginPlay`
  (`PrimitiveComponent.IgnoreActorWhenMoving` (`self.Sphere`) (`self.GetInstigator`) true)
  (`self.Travel To Target` :!label _label)
  (`KismetSystemLibrary.Delay` 0.5)
  (goto _label))

(event `self.ReceiveHit`
  (params (MyComp :type "PrimitiveComponent Object Reference") (Other :type "Actor Object Reference") (OtherComp :type "PrimitiveComponent Object Reference") (bSelfMoved :type Boolean) (HitLocation :type "Vector Structure") (HitNormal :type "Vector Structure") (NormalImpulse :type "Vector Structure") (Hit :type "HitResult Structure (by ref)"))
  (if true
    (`self.K2_DestroyActor` (`.HitActor` (`GameplayStatics.BreakHitResult` Hit)))
    (`self.K2_DestroyActor`)))

(event `self.ReceiveTick`
  (params (DeltaSeconds :type "Float (single-precision)"))
  (`self.SetLifeSpan` 1.0))

(fn `TargetFinding`
  (returns (HomingTarget :type "SceneComponent Object Reference"))
  (bind _outactors (`GameplayStatics.GetAllActorsOfClass` "/Game/PlaneTest/Targets_BP.Targets_BP_C"))
  (for _array_element _outactors
    (bind _returnvalue (`KismetMathLibrary.VSize` (- (`self.K2_GetActorLocation` _array_element) (`self.K2_GetActorLocation`))))
    (if (< _returnvalue (`self.ClosestDistance`))
      (set `self.ClosestDistance` _returnvalue)
      (bind _output_get (set `self.HomingTarget` _array_element))
      (`KismetSystemLibrary.PrintString` (`KismetSystemLibrary.GetDisplayName` _output_get))))
  (return (`self.GetComponentByClass` (`self.HomingTarget`) "/Script/Engine.SceneComponent")))

(fn `UserConstructionScript`)