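; Player biplane pawn with physics-driven arcade flight, which fires regular and homing projectiles and is destroyed on hit.
; Input axes apply pitch, yaw and roll torques to the Driver body, while Tick counters spin and adds downward force as gravity.
; A looping timer steps throttle from held inputs.
; CalculateSpeed eases velocity toward the throttle-scaled forward vector each tick, then repositions the camera from world X velocity.
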(event `self.ReceiveHit`
  (params (MyComp :type "PrimitiveComponent Object Reference") (Other :type "Actor Object Reference") (OtherComp :type "PrimitiveComponent Object Reference") (bSelfMoved :type Boolean) (HitLocation :type "Vector Structure") (HitNormal :type "Vector Structure") (NormalImpulse :type "Vector Structure") (Hit :type "HitResult Structure (by ref)"))
  ;[1 1 1] Destroy on collision
  (`self.K2_DestroyActor`))

(event `self.ReceiveTick`
  (params (DeltaSeconds :type "Float (single-precision)"))
  (bind _driver (`self.Driver`))
  ;[1 1 1] Gravity for the plane
  (`PrimitiveComponent.AddTorqueInDegrees` _driver (/ (`KismetMathLibrary.NegateVector` (`PrimitiveComponent.GetPhysicsAngularVelocityInDegrees` (`self.Driver`) "None")) 1.0) "None" true)
  (`PrimitiveComponent.AddForce` _driver (0.0 0.0 -1500.0) "None" true)
  (`self.CalculateSpeed`))

(event `InputAxis|Roll`
  (params (AxisValue :type "Float (single-precision)"))
  ;[1 1 1] Roll
  (`PrimitiveComponent.AddTorqueInDegrees` (`self.Driver`) (`KismetMathLibrary.VLerp` (0.0 0.0 0.0) (* (`SceneComponent.GetForwardVector` (`self.Driver`)) (* AxisValue (`self.Aircontrol`))) 0.1) "None" true))

(event `self.ReceiveBeginPlay`
  ;[1 1 1] Acceleration and Deacceleration
  (`KismetSystemLibrary.K2_SetTimer` null "ThrottleInput" 0.05 true))

(event `InputAction|ThrottleUp`
  (params (Key :type "Key Structure"))
  ;[1 1 1] Acceleration and Deacceleration
  (:`Pressed`
    (set `self.ThrottleUp` true))
  (:`Released`
    (set `self.ThrottleUp` false)))

(event `InputAction|ThrottleDown`
  (params (Key :type "Key Structure"))
  ;[1 1 1] Acceleration and Deacceleration
  (:`Pressed`
    (set `self.ThrottleDown` true))
  (:`Released`
    (set `self.ThrottleDown` false)))

(event `InputAxis|MoveRight`
  (params (AxisValue :type "Float (single-precision)"))
  ;[1 1 1] Yaw
  (`PrimitiveComponent.AddTorqueInDegrees` (`self.Driver`) (`KismetMathLibrary.VLerp` (0.0 0.0 0.0) (* (`SceneComponent.GetUpVector` (`self.Driver`)) (* AxisValue (`self.Aircontrol`))) 0.1) "None" true))

(event `InputAction|Shooting`
  (params (Key :type "Key Structure"))
  ;[1 1 1] Shooting
  (:`Pressed`
    (`|SpawnActorFromClass` "/Game/PlaneTest/Projectile_BP.Projectile_BP_C" (`SceneComponent.K2_GetComponentToWorld` (`self.Projectile_Spawn`)) "Undefined" "OverrideRootScale" null null)))

(event `InputAxis|MoveForward`
  (params (AxisValue :type "Float (single-precision)"))
  ;[1 1 1] Pitch
  (`PrimitiveComponent.AddTorqueInDegrees` (`self.Driver`) (`KismetMathLibrary.VLerp` (0.0 0.0 0.0) (* (`SceneComponent.GetRightVector` (`self.Driver`)) (* AxisValue (`self.Aircontrol`))) 0.1) "None" true))

(event `InputAction|Ability`
  (params (Key :type "Key Structure"))
  ;[1 1 1] Ability
  (:`Pressed`
    (`|SpawnActorFromClass` "/Game/PlaneTest/HomingProjectile_BP.HomingProjectile_BP_C" (`SceneComponent.K2_GetComponentToWorld` (`self.Projectile_Spawn`)) "Undefined" "OverrideRootScale" null null)))

(fn `CalculateSpeed`
  (bind _driver (`self.Driver`))
  ;[1 1 1] Speed calculation
  (bind _returnvalue (`PrimitiveComponent.GetPhysicsLinearVelocity` _driver "None"))
  (`PrimitiveComponent.SetPhysicsLinearVelocity` (`self.Driver`) (`KismetMathLibrary.VLerp` _returnvalue (* (`SceneComponent.GetForwardVector` _driver) (`KismetMathLibrary.FClamp` (* (`self.ThrottleAmount`) 250.0) 0.0 25000.0)) 0.01) false "None")
  (bind _returnvalue_2 (`PrimitiveComponent.GetPhysicsLinearVelocity` (`self.Driver`) "None"))
  ;[1 1 1] Camera movement related with speed
  (`SceneComponent.K2_SetRelativeLocation` (`self.Camera`) (* (+ (* (`KismetMathLibrary.Vector_GetAbs` _returnvalue_2) (0.1 0.0 0.0)) (`SceneComponent.RelativeLocation` (`self.Camera`))) (-1.0 0.0 0.0)) false false))

(fn `ThrottleInput`
  (bind _throttleamount (`self.ThrottleAmount`))
  ;[1 1 1] Increment and Deincrement acceleration
  (if (`self.ThrottleUp`)
    (bind _result (`/Engine/EditorBlueprintResources/StandardMacros.IncrementInt` _throttleamount)
      (:`  `
        (bind _output_get (set `self.ThrottleAmount` (`KismetMathLibrary.Clamp` _result 0 100)))
        (`KismetSystemLibrary.PrintString` (`KismetStringLibrary.Conv_IntToString` _output_get))))
    (elif (`self.ThrottleDown`)
      (bind _result_2 (`/Engine/EditorBlueprintResources/StandardMacros.DecrementInt` _throttleamount)
        (:`  `
          (bind _output_get_2 (set `self.ThrottleAmount` (`KismetMathLibrary.Clamp` _result_2 0 100)))
          (`KismetSystemLibrary.PrintString` (`KismetStringLibrary.Conv_IntToString` _output_get_2)))))))

(fn `UserConstructionScript`)